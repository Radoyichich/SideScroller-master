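; A platform that disappears shortly after the third-person character steps on it.
; A box overlap trigger swaps the floor material as a warning, then after a further delay hides the floor and disables its collision.
; Leaving the box starts a delayed reset that restores the original material, visibility and collision, without checking which actor left.
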(event OnComponentBeginOverlap(Box)
  (params (OverlappedComponent :type Primitive%20Component%20Object%20Reference) (OtherActor :type Actor%20Object%20Reference) (OtherComp :type Primitive%20Component%20Object%20Reference) (OtherBodyIndex :type Integer) (bFromSweep :type Boolean) (SweepResult :type Hit%20Result%20Structure%20%28by%20ref%29))
  (bind _floor (Variables|Default|GetFloor))
  (Utilities|Casting|CastToThirdPersonCharacter OtherActor)
  (Utilities|FlowControl|Delay 0.5)
  (Rendering|Material|SetMaterial _floor 0 "/Game/TP/StarterContent/Materials/M_Wood_Pine.M_Wood_Pine")
  (Utilities|FlowControl|Delay 1.0)
  (Rendering|SetVisibility _floor false false)
  (Collision|SetCollisionEnabled _floor "NoCollision"))

(event OnComponentEndOverlap(Box)
  (params (OverlappedComponent :type Primitive%20Component%20Object%20Reference) (OtherActor :type Actor%20Object%20Reference) (OtherComp :type Primitive%20Component%20Object%20Reference) (OtherBodyIndex :type Integer))
  (bind _floor (Variables|Default|GetFloor))
  (Utilities|FlowControl|Delay 5.0)
  (Rendering|Material|SetMaterial _floor 0 "/Game/TP/StarterContent/Materials/M_Wood_Oak.M_Wood_Oak")
  (Rendering|SetVisibility _floor true false)
  (Collision|SetCollisionEnabled _floor "QueryAndPhysics"))

(fn ConstructionScript)