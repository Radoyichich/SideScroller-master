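; Sliding door Blueprint that opens when the player's ThirdPersonCharacter enters its trigger box and closes when it leaves.
; Box overlap begin and end events play the DoorSlide timeline forward or in reverse, each with its own sound at the door's location.
; The timeline's Slide track drives a Lerp that moves the SlidingDoor component along its local Y axis.
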(event OnComponentBeginOverlap(Box)
  (params (OverlappedComponent :type Primitive%20Component%20Object%20Reference) (OtherActor :type Actor%20Object%20Reference) (OtherComp :type Primitive%20Component%20Object%20Reference) (OtherBodyIndex :type Integer) (bFromSweep :type Boolean) (SweepResult :type Hit%20Result%20Structure%20%28by%20ref%29))
  (Utilities|Casting|CastToThirdPersonCharacter OtherActor)
  (Audio|PlaySoundatLocation "/Game/Blueprints/Door/SlidingDoor.SlidingDoor" (Transformation|GetActorLocation) "0, 0, 0" 1.0 1.0 0.0 0 0 0)
  (bind _slide (Timeline|DoorSlide Play)
    (:Update
      (Transformation|SetRelativeLocation (Variables|Default|GetSlidingDoor) (Math|Vector|MakeVector 0.0 (Math|Float|Lerp 0.0 1.1e+02 _slide) 0.0) false false))))

(event OnComponentEndOverlap(Box)
  (params (OverlappedComponent :type Primitive%20Component%20Object%20Reference) (OtherActor :type Actor%20Object%20Reference) (OtherComp :type Primitive%20Component%20Object%20Reference) (OtherBodyIndex :type Integer))
  (Utilities|Casting|CastToThirdPersonCharacter OtherActor)
  (Audio|PlaySoundatLocation "/Game/Blueprints/Door/SlidingDoorClose.SlidingDoorClose" (Transformation|GetActorLocation) "0, 0, 0" 1.0 1.0 0.0 0 0 0)
  (bind _slide (Timeline|DoorSlide Reverse)
    (:Update
      (Transformation|SetRelativeLocation (Variables|Default|GetSlidingDoor) (Math|Vector|MakeVector 0.0 (Math|Float|Lerp 0.0 1.1e+02 _slide) 0.0) false false))))

(fn ConstructionScript)