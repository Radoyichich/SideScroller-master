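; Warning note actor that lets the player show and hide a warning widget with the Interact key while standing in its box.
; Box overlap by the ThirdPersonCharacter enables input on the actor and opens a gate, which is never closed again.
; Interact passes through the gate to a FlipFlop that alternately creates and removes the Warning_Widget.
; Leaving the box disables input and removes the widget, without resetting the FlipFlop.
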(event OnComponentBeginOverlap(Box)
  (params (OverlappedComponent :type Primitive%20Component%20Object%20Reference) (OtherActor :type Actor%20Object%20Reference) (OtherComp :type Primitive%20Component%20Object%20Reference) (OtherBodyIndex :type Integer) (bFromSweep :type Boolean) (SweepResult :type Hit%20Result%20Structure%20%28by%20ref%29))
  (Utilities|Casting|CastToThirdPersonCharacter OtherActor)
  (Input|EnableInput (Game|GetPlayerController 0))
  (Utilities|FlowControl|Gate true) ; enters at Open
)

(event OnComponentEndOverlap(Box)
  (params (OverlappedComponent :type Primitive%20Component%20Object%20Reference) (OtherActor :type Actor%20Object%20Reference) (OtherComp :type Primitive%20Component%20Object%20Reference) (OtherBodyIndex :type Integer))
  (Utilities|Casting|CastToThirdPersonCharacter OtherActor)
  (Input|DisableInput (Game|GetPlayerController 0))
  (Widget|RemovefromParent (stale Input|ActionEvents|InputActionInteract _returnvalue)))

(event Input|ActionEvents|InputActionInteract
  (params (Key :type Key%20Structure))
  (:Pressed
    (Utilities|FlowControl|Gate true
      (:Exit
        (Utilities|FlowControl|FlipFlop
          (:A
            (bind _returnvalue (UserInterface|CreateWidget "/Game/Blueprints/Notes/Warning_Widget.Warning_Widget_C"))
            (UserInterface|Viewport|AddtoViewport _returnvalue 0))
          (:B
            (Widget|RemovefromParent _returnvalue)))))))

(fn ConstructionScript)