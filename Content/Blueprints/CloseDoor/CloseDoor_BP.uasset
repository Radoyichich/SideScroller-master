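; CloseDoor_BP is a trigger actor that slides a door to a set position when the third-person character enters its box.
; It caches the door's relative location at BeginPlay, then a timeline lerps from there to End without sweep.
; The Duration variable feeds the timeline's play rate directly, so higher values move the door faster.
; The timeline only plays forward, with no reverse or end-overlap handling.
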(event OnComponentBeginOverlap(Box)
  (params (OverlappedComponent :type Primitive%20Component%20Object%20Reference) (OtherActor :type Actor%20Object%20Reference) (OtherComp :type Primitive%20Component%20Object%20Reference) (OtherBodyIndex :type Integer) (bFromSweep :type Boolean) (SweepResult :type Hit%20Result%20Structure%20%28by%20ref%29))
  (Utilities|Casting|CastToThirdPersonCharacter OtherActor)
  (Components|Timeline|SetPlayRate (Variables|Default|GetCloseDoor) (Variables|Default|GetDuration))
  (bind _movedoor (Timeline|CloseDoor Play)
    (:Update
      (Transformation|SetRelativeLocation (Variables|Default|GetDoor) (Math|Vector|Lerp(Vector) (Variables|Default|GetStart) (Variables|Default|GetEnd) _movedoor) false false))))

(event EventBeginPlay
  (Variables|Default|SetStart (Variables|/Script/Engine.SceneComponent|GetRelativeLocation (Variables|Default|GetDoor))))

(fn ConstructionScript)