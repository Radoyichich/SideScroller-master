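; Trigger volume that makes assigned HiddenObjects translucent while a ThirdPersonCharacter is inside its Box.
; On overlap, a timeline swaps each static mesh's first material for a MaterialToChange dynamic instance and lowers its Opacity.
; Each fade-out update also appends the current materials to SourceMaterials, which is never cleared.
; On exit, a second timeline partly raises Opacity, then rebuilds materials from SourceMaterials by running index when finished.
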(event OnComponentBeginOverlap(Box)
  (params (OverlappedComponent :type Primitive%20Component%20Object%20Reference) (OtherActor :type Actor%20Object%20Reference) (OtherComp :type Primitive%20Component%20Object%20Reference) (OtherBodyIndex :type Integer) (bFromSweep :type Boolean) (SweepResult :type Hit%20Result%20Structure%20%28by%20ref%29))
  (Utilities|Casting|CastToThirdPersonCharacter OtherActor)
  (if (Utilities|Array|IsValidIndex (Variables|Default|GetHiddenObjects))
    (bind _alpha (Timeline|FadeOut_TL PlayFromStart)
      (:Update
        (for _array_element (Variables|Default|GetHiddenObjects)
          (for _array_element_2 (Actor|GetComponentsByClass _array_element "/Script/Engine.StaticMeshComponent")
            (Utilities|Array|Add (Variables|Default|GetSourceMaterials) (Rendering|Material|GetMaterial _array_element_2 0))
            (bind _returnvalue (Rendering|Material|CreateDynamicMaterialInstance _array_element_2 0 (Variables|Default|GetMaterialToChange) "None" :!class /Script/Engine.PrimitiveComponent))
            (Rendering|Material|SetScalarParameterValue _returnvalue "Opacity" (Math|Float|Lerp 1.0 0.25 _alpha) :!class /Script/Engine.MaterialInstanceDynamic)))))))

(event OnComponentEndOverlap(Box)
  (params (OverlappedComponent :type Primitive%20Component%20Object%20Reference) (OtherActor :type Actor%20Object%20Reference) (OtherComp :type Primitive%20Component%20Object%20Reference) (OtherBodyIndex :type Integer))
  (Variables|Default|SetCounter 0)
  (Utilities|Casting|CastToThirdPersonCharacter OtherActor)
  (if (Utilities|Array|IsValidIndex (Variables|Default|GetHiddenObjects))
    (bind _alpha (Timeline|FadeIn_TL PlayFromStart)
      (:Update
        (for _array_element (Variables|Default|GetHiddenObjects)
          (for _array_element_2 (Actor|GetComponentsByClass _array_element "/Script/Engine.StaticMeshComponent")
            (Rendering|Material|SetScalarParameterValueonMaterials _array_element_2 "Opacity" (Math|Float|Lerp 0.5 0.75 _alpha)))))
      (:Finished
        (for _array_element_3 (Variables|Default|GetHiddenObjects)
          (for _array_element_4 (Actor|GetComponentsByClass _array_element_3 "/Script/Engine.StaticMeshComponent")
            (Rendering|Material|CreateDynamicMaterialInstance _array_element_4 0 (Utilities|Array|Get(acopy) (Variables|Default|GetSourceMaterials) (Variables|Default|GetCounter)) "None" :!class /Script/Engine.PrimitiveComponent)
            (Math|Integer|IncrementInt (Variables|Default|GetCounter))))))))

(fn ConstructionScript)