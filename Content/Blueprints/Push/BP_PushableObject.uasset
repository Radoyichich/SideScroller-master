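; Pushable object actor that a character can take hold of to start pushing from predefined grip points, each shown by an arrow component.
; On Hold, it picks the closest push transform within the character's PushComponent range.
; Capsule and line traces check for standing room, walkable floor and walls between object and character.
; If clear, it snaps the character to that point and calls BeginPush, otherwise printing the failure reason.
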(event EventHold
  (params (Character :type Character%20Object%20Reference))
  (CallFunction|HundleInteractiom Character))

(fn ConstructionScript
  (Components|StaticMesh|SetStaticMesh (Variables|Default|GetStaticMesh) (Variables|Default|GetNewMesh))
  (for _array_element (Variables|Default|GetPushTransform)
    (AddComponent|AddArrowComponent false _array_element)))

(fn HundleInteractiom
  (params (Character :type Character%20Object%20Reference))
  (bind _returnvalue (Actor|GetComponentbyClass Character "/Game/Blueprints/Push/PushComponent.PushComponent_C"))
  (bind _capsulecomponent (Variables|/Script/Engine.Character|GetCapsuleComponent Character))
  (Utilities|IsValid Character
    (:Is%20Valid
      (Utilities|IsValid _returnvalue
        (:Is%20Valid
          (LocalVariables|SetPushComponent _returnvalue)
          (bind _bestindex (CallFunction|FindClosestPushTransformIndex (Math|Conversions|ToVector2D(Vector) (Transformation|GetActorLocation Character)) (Variables|/Game/Blueprints/Push/PushComponent.PushComponent_C|GetPushRange (LocalVariables|GetPushComponent))))
          (if (>= _bestindex 0)
            (LocalVariables|SetCharacterNewTransform (Math|Transform|MakeTransform (+ (.location (Math|Transform|ComposeTransforms (Utilities|Array|Get(acopy) (Variables|Default|GetPushTransform) _bestindex) (Transformation|GetActorTransform))) (Math|Vector|MakeVector 0.0 0.0 (Components|Capsule|GetScaledCapsuleHalfHeight (Variables|/Script/Engine.Character|GetCapsuleComponent Character)))) (.rotation (Math|Transform|ComposeTransforms (Utilities|Array|Get(acopy) (Variables|Default|GetPushTransform) _bestindex) (Transformation|GetActorTransform))) (.scale (Transformation|GetActorTransform Character))))
            (bind _outhit (Collision|CapsuleTraceByChannel (+ (.location (LocalVariables|GetCharacterNewTransform)) "0,0.000000,70.000000") (- (.location (LocalVariables|GetCharacterNewTransform)) "0, 0,110.000000") (Components|Capsule|GetScaledCapsuleRadius _capsulecomponent) (Components|Capsule|GetScaledCapsuleHalfHeight _capsulecomponent) "TraceTypeQuery1" false 0 "None"))
            (if (not (.binitialoverlap _outhit))
              (if (< (Class|CharacterMovementComponent|GetWalkableFloorZ (Variables|/Script/Engine.Character|GetCharacterMovement Character)) (.Z (Math|Vector|BreakVector (.impactnormal _outhit))))
                (bind _returnvalue_2 (Collision|LineTraceByChannel (Transformation|GetActorLocation) (.location (LocalVariables|GetCharacterNewTransform)) "TraceTypeQuery1" false (Utilities|Array|MakeArray Character) "None"))
                (if (not _returnvalue_2)
                  (Transformation|SetActorTransform Character (LocalVariables|GetCharacterNewTransform))
                  (Default|BeginPush (LocalVariables|GetPushComponent) self)
                  (else
                    (Development|PrintString "Walls Between Character and Object")))
                (else
                  (Development|PrintString "Floor Is Not Walkable")))
              (else
                (Development|PrintString "No Room To Stand")))
            (else
              (Development|PrintString "Push Transform Not Found"))))
        (:Is%20Not%20Valid
          (Development|PrintString "Push Component is Not Valid"))))
    (:Is%20Not%20Valid
      (Development|PrintString "Character is Not Valid"))))

(fn FindClosestPushTransformIndex
  (params (CharacterLocation :type Vector%202D%20Structure) (PushRange :type Float%20%28single-precision%29))
  (for (_array_element _array_index) (Variables|Default|GetPushTransform)
    (LocalVariables|SetCurrentTransformIndex _array_index)
    (LocalVariables|SetCurrentDistanceSq (Class|KismetMathLibrary|DistanceSquared2D (Math|Conversions|ToVector2D(Vector) (Math|Transform|TransformLocation (Transformation|GetActorTransform) (.location _array_element))) CharacterLocation))
    (if (< (LocalVariables|GetCurrentDistanceSq) (Math|Float|Square PushRange))
      (if (or (< (LocalVariables|GetCurrentDistanceSq) (LocalVariables|GetClosestDistanceSq)) (< (LocalVariables|GetClosestTransformIndex) 0))
        (LocalVariables|SetClosestTransformIndex (LocalVariables|GetCurrentTransformIndex))
        (LocalVariables|SetClosestDistanceSq (LocalVariables|GetCurrentDistanceSq)))))
  (return (LocalVariables|GetClosestTransformIndex)))