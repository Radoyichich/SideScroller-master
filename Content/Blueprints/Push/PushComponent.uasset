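; Character component that lets the player grab and push or pull objects, with the character attached to the object.
; BeginPush and EndPush toggle tick, attachment, pawn collision and orient-to-movement.
; Tick remaps move input by four yaw quadrants and offsets the object without sweep, using capsule and side line traces to clamp blocked directions.
; It also exposes push rotation, velocity, moving state and object height relative to the character's feet.
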(event EventBeginPlay
  (Components|Tick|SetComponentTickEnabled false)
  (bind _ascharacter (Utilities|Casting|CastToCharacter (Components|GetOwner)))
  (Variables|Default|SetCharacter _ascharacter))

(event EventTick
  (params (DeltaSeconds :type Float%20%28single-precision%29))
  (bind _character (Variables|Default|GetCharacter))
  (bind _character_2 (Variables|Default|GetCharacter))
  (bind _character_3 (Variables|Default|GetCharacter))
  (bind _character_4 (Variables|Default|GetCharacter))
  (bind _character_5 (Variables|Default|GetCharacter))
  (bind _character_6 (Variables|Default|GetCharacter))
  (bind _character_7 (Variables|Default|GetCharacter))
  (bind _character_8 (Variables|Default|GetCharacter))
  (bind _character_9 (Variables|Default|GetCharacter))
  (bind _character_10 (Variables|Default|GetCharacter))
  (bind _character_11 (Variables|Default|GetCharacter))
  (bind _character_12 (Variables|Default|GetCharacter))
  (bind _returnvalue (Transformation|GetActorLocation _character_11))
  (bind _returnvalue_2 (Transformation|GetActorRotation _character_11))
  (bind _returnvalue_3 (Transformation|GetActorLocation _character_12))
  (bind _returnvalue_4 (Transformation|GetActorRotation _character_12))
  (bind _returnvalue_5 (Transformation|GetActorLocation _character))
  (bind _returnvalue_6 (Transformation|GetActorLocation _character_2))
  (bind _returnvalue_7 (Transformation|GetActorLocation _character_3))
  (bind _returnvalue_8 (Transformation|GetActorLocation _character_4))
  (bind _returnvalue_9 (Transformation|GetActorLocation _character_5))
  (bind _returnvalue_10 (Transformation|GetActorRotation _character_5))
  (bind _returnvalue_11 (Transformation|GetActorLocation _character_6))
  (bind _returnvalue_12 (Transformation|GetActorRotation _character_6))
  (bind _returnvalue_13 (Transformation|GetActorLocation _character_7))
  (bind _returnvalue_14 (Transformation|GetActorRotation _character_7))
  (bind _returnvalue_15 (Transformation|GetActorLocation _character_8))
  (bind _returnvalue_16 (Transformation|GetActorRotation _character_8))
  (bind _returnvalue_17 (Transformation|GetActorLocation _character_9))
  (bind _returnvalue_18 (Transformation|GetActorRotation _character_9))
  (bind _returnvalue_19 (Transformation|GetActorLocation _character_10))
  (bind _returnvalue_20 (Transformation|GetActorRotation _character_10))
  (Utilities|FlowControl|Sequence
    (:then_0
      (Utilities|FlowControl|Sequence
        (:then_0
          (if (not (Variables|Default|GetCanMoveRight))
            (Variables|Default|SetRightMove (Math|Float|Clamp(Float) (Variables|Default|GetRightMove)))))
        (:then_1
          (if (not (Variables|Default|GetCanMoveLeft))
            (Variables|Default|SetRightMove (Math|Float|Clamp(Float) (Variables|Default|GetRightMove) -1.0 0.0))))
        (:then_2
          (if (not (Variables|Default|GetCanMoveUp))
            (Variables|Default|SetForwardMove (Math|Float|Clamp(Float) (Variables|Default|GetForwardMove)))))
        (:then_3
          (if (not (Variables|Default|GetCanMoveDown))
            (Variables|Default|SetForwardMove (Math|Float|Clamp(Float) (Variables|Default|GetForwardMove) -1.0 0.0))))))
    (:then_1
      (Variables|Default|SetCurrentActorZRotation (.yaw (Transformation|GetActorRotation (Variables|Default|GetCharacter))))
      ;[1 1 1] Up
      (if (and (< (Variables|Default|GetCurrentActorZRotation) 8e+01) (>= (Variables|Default|GetCurrentActorZRotation) 0.0))
        (bind _currentpushableobject (Variables|Default|GetCurrentPushableObject)
          (:then
            (Transformation|AddActorWorldOffset _currentpushableobject (CallFunction|GetDeltaLocation DeltaSeconds (Variables|Default|GetForwardMove) (Variables|Default|GetRightMove)))
            (Variables|Default|SetPushRotation (Math|Rotator|MakeRotfromX (CallFunction|GetDeltaLocation DeltaSeconds (Variables|Default|GetForwardMove) (Variables|Default|GetRightMove))))
            (Variables|Default|SetPushVelocity (Math|Vector|MakeVector (Variables|Default|GetPushSpeed) 0.0 0.0))
            (bind _returnvalue_21 (Collision|CapsuleTraceByChannel _returnvalue_6 _returnvalue_6 42.0 96.0 "TraceTypeQuery1" false 0 "ForOneFrame"))
            (if _returnvalue_21
              (Variables|Default|SetCanMoveUp false)
              (else
                (Variables|Default|SetCanMoveUp true)))
            (Utilities|FlowControl|Sequence
              (:then_0
                (bind _returnvalue_22 (Collision|LineTraceByChannel _returnvalue_15 (+ _returnvalue_15 (* (Math|Vector|GetForwardVector (Math|Rotator|MakeRotator (.roll _returnvalue_16) (.pitch _returnvalue_16) (+ (.yaw _returnvalue_16) -9e+01))) 6e+01)) "TraceTypeQuery1" false 0 "ForOneFrame"))
                (if _returnvalue_22
                  (Variables|Default|SetCanMoveRight false)
                  (else
                    (Variables|Default|SetCanMoveRight true))))
              (:then_1
                (bind _returnvalue_23 (Collision|LineTraceByChannel _returnvalue_13 (+ _returnvalue_13 (* (Math|Vector|GetForwardVector (Math|Rotator|MakeRotator (.roll _returnvalue_14) (.pitch _returnvalue_14) (+ (.yaw _returnvalue_14) 9e+01))) 6e+01)) "TraceTypeQuery1" false 0 "ForOneFrame" true "(R=1.000000,G=0.879006,B=0.000000,A=1.000000)"))
                (if _returnvalue_23
                  (Variables|Default|SetCanMoveLeft false)
                  (else
                    (Variables|Default|SetCanMoveLeft true))))))
          (:else))
        (else
          ;[1 1 1] Right
          (if (and (< (Variables|Default|GetCurrentActorZRotation) 1.7e+02) (>= (Variables|Default|GetCurrentActorZRotation) 8e+01))
            (bind _currentpushableobject_2 (Variables|Default|GetCurrentPushableObject)
              (:then
                (Transformation|AddActorWorldOffset _currentpushableobject_2 (CallFunction|GetDeltaLocation DeltaSeconds (Variables|Default|GetRightMove) (* (Variables|Default|GetForwardMove) -1.0)))
                (Variables|Default|SetPushRotation (Math|Rotator|MakeRotfromX (CallFunction|GetDeltaLocation DeltaSeconds (Variables|Default|GetRightMove) (* (Variables|Default|GetForwardMove) -1.0))))
                (Variables|Default|SetPushVelocity (Math|Vector|MakeVector 0.0 (Variables|Default|GetPushSpeed) 0.0))
                (bind _returnvalue_24 (Collision|CapsuleTraceByChannel _returnvalue_7 _returnvalue_7 42.0 96.0 "TraceTypeQuery1" false 0 "ForOneFrame"))
                (if _returnvalue_24
                  (Variables|Default|SetCanMoveRight false)
                  (else
                    (Variables|Default|SetCanMoveRight true)))
                (Utilities|FlowControl|Sequence
                  (:then_0
                    (bind _returnvalue_25 (Collision|LineTraceByChannel _returnvalue_19 (+ _returnvalue_19 (* (Math|Vector|GetForwardVector (Math|Rotator|MakeRotator (.roll _returnvalue_20) (.pitch _returnvalue_20) (+ (.yaw _returnvalue_20) -9e+01))) 6e+01)) "TraceTypeQuery1" false 0 "ForOneFrame"))
                    (if _returnvalue_25
                      (Variables|Default|SetCanMoveDown false)
                      (else
                        (Variables|Default|SetCanMoveDown true))))
                  (:then_1
                    (bind _returnvalue_26 (Collision|LineTraceByChannel _returnvalue_17 (+ _returnvalue_17 (* (Math|Vector|GetForwardVector (Math|Rotator|MakeRotator (.roll _returnvalue_18) (.pitch _returnvalue_18) (+ (.yaw _returnvalue_18) 9e+01))) 6e+01)) "TraceTypeQuery1" false 0 "ForOneFrame" true "(R=1.000000,G=0.879006,B=0.000000,A=1.000000)"))
                    (if _returnvalue_26
                      (Variables|Default|SetCanMoveUp false)
                      (else
                        (Variables|Default|SetCanMoveUp true))))))
              (:else))
            (else
              ;[1 1 1] Left
              (if (and (< (Variables|Default|GetCurrentActorZRotation) 0.0) (>= (Variables|Default|GetCurrentActorZRotation) -95.0))
                (bind _currentpushableobject_3 (Variables|Default|GetCurrentPushableObject)
                  (:then
                    (Transformation|AddActorWorldOffset _currentpushableobject_3 (CallFunction|GetDeltaLocation DeltaSeconds (* (Variables|Default|GetRightMove) -1.0) (Variables|Default|GetForwardMove)))
                    (Variables|Default|SetPushRotation (Math|Rotator|MakeRotfromX (CallFunction|GetDeltaLocation DeltaSeconds (* (Variables|Default|GetRightMove) -1.0) (Variables|Default|GetForwardMove))))
                    (Variables|Default|SetPushVelocity (Math|Vector|MakeVector 0.0 (* (Variables|Default|GetPushSpeed) -1.0) 0.0))
                    (bind _returnvalue_27 (Collision|CapsuleTraceByChannel _returnvalue_8 _returnvalue_8 42.0 96.0 "TraceTypeQuery1" false 0 "ForOneFrame"))
                    (if _returnvalue_27
                      (Variables|Default|SetCanMoveLeft false)
                      (else
                        (Variables|Default|SetCanMoveLeft true)))
                    (Utilities|FlowControl|Sequence
                      (:then_0
                        (bind _returnvalue_28 (Collision|LineTraceByChannel _returnvalue_3 (+ _returnvalue_3 (* (Math|Vector|GetForwardVector (Math|Rotator|MakeRotator (.roll _returnvalue_4) (.pitch _returnvalue_4) (+ (.yaw _returnvalue_4) -9e+01))) 6e+01)) "TraceTypeQuery1" false 0 "ForOneFrame"))
                        (if _returnvalue_28
                          (Variables|Default|SetCanMoveUp false)
                          (else
                            (Variables|Default|SetCanMoveUp true))))
                      (:then_1
                        (bind _returnvalue_29 (Collision|LineTraceByChannel _returnvalue (+ _returnvalue (* (Math|Vector|GetForwardVector (Math|Rotator|MakeRotator (.roll _returnvalue_2) (.pitch _returnvalue_2) (+ (.yaw _returnvalue_2) 9e+01))) 6e+01)) "TraceTypeQuery1" false 0 "ForOneFrame" true "(R=1.000000,G=0.879006,B=0.000000,A=1.000000)"))
                        (if _returnvalue_29
                          (Variables|Default|SetCanMoveDown false)
                          (else
                            (Variables|Default|SetCanMoveDown true))))))
                  (:else))
                (else
                  ;[1 1 1] Down
                  (if (and (< (Variables|Default|GetCurrentActorZRotation) -95.0) (>= (Variables|Default|GetCurrentActorZRotation) -1.8e+02))
                    (bind _currentpushableobject_4 (Variables|Default|GetCurrentPushableObject)
                      (:then
                        (Transformation|AddActorWorldOffset _currentpushableobject_4 (CallFunction|GetDeltaLocation DeltaSeconds (* (Variables|Default|GetForwardMove) -1.0) (* (Variables|Default|GetRightMove) -1.0)))
                        (Variables|Default|SetPushRotation (Math|Rotator|MakeRotfromX (CallFunction|GetDeltaLocation DeltaSeconds (* (Variables|Default|GetForwardMove) -1.0) (* (Variables|Default|GetRightMove) -1.0))))
                        (Variables|Default|SetPushVelocity (Math|Vector|MakeVector (* (Variables|Default|GetPushSpeed) -1.0) 0.0 0.0))
                        (bind _returnvalue_30 (Collision|CapsuleTraceByChannel _returnvalue_5 _returnvalue_5 42.0 96.0 "TraceTypeQuery1" false 0 "ForOneFrame"))
                        (if _returnvalue_30
                          (Variables|Default|SetCanMoveDown false)
                          (else
                            (Variables|Default|SetCanMoveDown true)))
                        (Utilities|FlowControl|Sequence
                          (:then_0
                            (bind _returnvalue_31 (Collision|LineTraceByChannel _returnvalue_9 (+ _returnvalue_9 (* (Math|Vector|GetForwardVector (Math|Rotator|MakeRotator (.roll _returnvalue_10) (.pitch _returnvalue_10) (+ (.yaw _returnvalue_10) -9e+01))) 6e+01)) "TraceTypeQuery1" false 0 "ForOneFrame"))
                            (if _returnvalue_31
                              (Variables|Default|SetCanMoveLeft false)
                              (else
                                (Variables|Default|SetCanMoveLeft true))))
                          (:then_1
                            (bind _returnvalue_32 (Collision|LineTraceByChannel _returnvalue_11 (+ _returnvalue_11 (* (Math|Vector|GetForwardVector (Math|Rotator|MakeRotator (.roll _returnvalue_12) (.pitch _returnvalue_12) (+ (.yaw _returnvalue_12) 9e+01))) 6e+01)) "TraceTypeQuery1" false 0 "ForOneFrame" true "(R=1.000000,G=0.879006,B=0.000000,A=1.000000)"))
                            (if _returnvalue_32
                              (Variables|Default|SetCanMoveRight false)
                              (else
                                (Variables|Default|SetCanMoveRight true))))))
                      (:else))))))))))))

(fn BeginPush
  (params (Pushable%20Object :type BP%20Pushable%20Object%20Object%20Reference))
  (bind _character (Variables|Default|GetCharacter))
  (Variables|Default|GetCurrentPushableObject
    (:then)
    (:else
      (bind _output_get (Variables|Default|SetCurrentPushableObject Pushable%20Object))
      (Transformation|AttachActorToActor _character _output_get "None" "KeepWorld" "KeepWorld" "KeepWorld" true)
      (Variables|/Script/Engine.CharacterMovementComponent|SetbOrientRotationToMovement (Variables|/Script/Engine.Character|GetCharacterMovement _character) false)
      (Components|Tick|SetComponentTickEnabled true)
      (Collision|SetCollisionResponsetoChannel (Variables|/Game/Blueprints/Push/BP_PushableObject.BP_PushableObject_C|GetStaticMesh (Variables|Default|GetCurrentPushableObject)) "ECC_Pawn" "ECR_Ignore"))))

(fn EndPush
  (bind _character (Variables|Default|GetCharacter))
  (Variables|Default|SetCanMoveRight true)
  (Variables|Default|SetCanMoveLeft true)
  (Variables|Default|SetCanMoveUp true)
  (Variables|Default|SetCanMoveDown true)
  (Variables|Default|GetCurrentPushableObject
    (:then
      (Collision|SetCollisionResponsetoChannel (Variables|/Game/Blueprints/Push/BP_PushableObject.BP_PushableObject_C|GetStaticMesh (Variables|Default|GetCurrentPushableObject)) "ECC_Pawn" "ECR_Block")
      (Variables|Default|SetCurrentPushableObject 0)
      (Variables|Default|SetIsMovingAnObject false)
      (Transformation|DetachFromActor _character "KeepWorld" "KeepWorld" "KeepWorld")
      (Variables|/Script/Engine.CharacterMovementComponent|SetbOrientRotationToMovement (Variables|/Script/Engine.Character|GetCharacterMovement _character) true)
      (Components|Tick|SetComponentTickEnabled false))
    (:else)))

(fn IsHoldingObject
  (return (Utilities|IsValid (Variables|Default|GetCurrentPushableObject))))

(fn GetDeltaLocation
  (params (DeltaSecond :type Float%20%28single-precision%29) (ForwardMove :type Float%20%28single-precision%29) (RightMove :type Float%20%28single-precision%29))
  (Variables|Default|SetIsMovingAnObject (or (!= ForwardMove 0.0) (!= RightMove 0.0)))
  (return (+ (* (* (Transformation|GetActorForwardVector (Variables|Default|GetCharacter)) ForwardMove) (* DeltaSecond (Variables|Default|GetPushSpeed))) (* (* (Transformation|GetActorRightVector (Variables|Default|GetCharacter)) RightMove) (* (Variables|Default|GetPushSpeed) DeltaSecond)))))

(fn GetPushableHeight
  (bind _character (Variables|Default|GetCharacter))
  (Utilities|FlowControl|Sequence
    (:then_0
      (bind _currentpushableobject (Variables|Default|GetCurrentPushableObject)
        (:then
          (if (== (Variables|/Game/Blueprints/Push/BP_PushableObject.BP_PushableObject_C|GetCustomHeight _currentpushableobject) 0.0)
            (LocalVariables|SetTopOfObject (+ (.z (.BoxExtent (Collision|GetComponentBounds (Variables|/Game/Blueprints/Push/BP_PushableObject.BP_PushableObject_C|GetStaticMesh _currentpushableobject)))) (.z (Transformation|GetActorLocation (Variables|Default|GetCurrentPushableObject)))))
            (LocalVariables|SetFeetOfCharacter (- (.z (Transformation|GetActorLocation _character)) (Components|Capsule|GetScaledCapsuleHalfHeight (Variables|/Script/Engine.Character|GetCapsuleComponent _character))))
            (return (- (LocalVariables|GetTopOfObject) (LocalVariables|GetFeetOfCharacter)))
            (else
              (return (Variables|/Game/Blueprints/Push/BP_PushableObject.BP_PushableObject_C|GetCustomHeight _currentpushableobject)))))
        (:else)))
    (:then_1
      (return 0.0))))