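; ActiveCamera is a camera actor that tracks the player character, rotating its camera component to look at it every tick.
; The player's distance, normalized between min and max bounds, blends the field of view between near and far values with smoothed interpolation.
; The actor also slides smoothly along world Y only, easing toward the midpoint between itself and the player while keeping X and Z fixed.
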(event EventBeginPlay
  (Variables|Default|SetTargetActor (Game|GetPlayerCharacter 0)))

(event EventTick
  (params (DeltaSeconds :type Float%20%28single-precision%29))
  (bind _returnvalue (Transformation|GetActorLocation))
  (bind _cameracomponent (Variables|CameraActor|GetCameraComponent))
  (bind (_x _y _z) (Math|Vector|BreakVector _returnvalue))
  ;[1 1 1] Update Camera Rotation/Look at
  (Transformation|SetWorldRotation (Variables|CameraActor|GetCameraComponent) (Math|Rotator|FindLookatRotation (Transformation|GetActorLocation) (Transformation|GetActorLocation (Variables|Default|GetTargetActor))) false false)
  ;[1 1 1] Get Player Distance
  (Variables|Default|SetTargetDistance (Transformation|GetDistanceTo (Variables|Default|GetTargetActor)))
  ;[1 1 1] Normalize Distance
  (Variables|Default|SetCurrentDistanceAlfa (Math|Float|Clamp(Float) (Math|Float|NormalizetoRange (Variables|Default|GetTargetDistance) (Variables|Default|GetMinDistance) (Variables|Default|GetMaxDistance))))
  ;[1 1 1] Set FOV
  (Camera|SetFieldOfView _cameracomponent (Math|Interpolation|FInterpTo (Variables|/Script/Engine.CameraComponent|GetFieldOfView _cameracomponent) (Math|Float|Lerp (Variables|Default|GetNearFOV) (Variables|Default|GetFarFOV) (Variables|Default|GetCurrentDistanceAlfa)) (Utilities|Time|GetWorldDeltaSeconds) (Variables|Default|GetFOVSpeed)))
  ;[1 1 1] Set Camera Location
  (Transformation|SetActorLocation (Math|Interpolation|VInterpTo _returnvalue (Math|Vector|MakeVector _x (.y (Math|Vector|Lerp(Vector) (Transformation|GetActorLocation (Variables|Default|GetTargetActor)) _returnvalue 0.5)) _z) (Utilities|Time|GetWorldDeltaSeconds) (Variables|Default|GetCameraSpeed)) false false))

(fn ConstructionScript)