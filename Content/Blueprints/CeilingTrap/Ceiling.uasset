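; Falling ceiling trap that kills the player on contact and restarts the level.
; On BeginPlay the Ceiling timeline lerps the mesh's relative location from Start to End without sweeping, using Duration as play rate, so higher values move it faster.
; When a ThirdPersonCharacter overlaps the Box, it ragdolls and loses input.
; After a short delay the camera and audio fade out, then the current level reopens by name.
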(event OnComponentBeginOverlap(Box)
  (params (OverlappedComponent :type Primitive%20Component%20Object%20Reference) (OtherActor :type Actor%20Object%20Reference) (OtherComp :type Primitive%20Component%20Object%20Reference) (OtherBodyIndex :type Integer) (bFromSweep :type Boolean) (SweepResult :type Hit%20Result%20Structure%20%28by%20ref%29))
  (bind _asthird_person_character (Utilities|Casting|CastToThirdPersonCharacter OtherActor))
  (Default|PlayRagdoll _asthird_person_character)
  (Input|DisableInput _asthird_person_character 0)
  (Utilities|FlowControl|Delay 1.0)
  (CameraFades|StartCameraFade :self (Game|GetPlayerCameraManager 0) :ToAlpha 1.0 :Duration 2.0 :bShouldFadeAudio true :bHoldWhenFinished true)
  (Utilities|FlowControl|Delay 2.1)
  (bind _returnvalue (Game|GetCurrentLevelName true))
  (Game|OpenLevel(byName) (Utilities|String|StringToName _returnvalue)))

(event EventBeginPlay
  (Components|Timeline|SetPlayRate (Variables|Default|GetCeiling) (Variables|Default|GetDuration))
  (bind _falling (Timeline|Ceiling Play)
    (:Update
      (Transformation|SetRelativeLocation (Variables|Default|GetStaticMesh) (Math|Vector|Lerp(Vector) (Variables|Default|GetStart) (Variables|Default|GetEnd) _falling) false false))))

(fn ConstructionScript)